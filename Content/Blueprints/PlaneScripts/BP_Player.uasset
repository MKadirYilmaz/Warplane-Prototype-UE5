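; BP_Player is the player aircraft Blueprint, animating landing gear and control surfaces through the G_PlaneAnimBP animation instance on AircraftMesh.
; OnOffGears toggles a gear flag with a FlipFlop, and Tick steps the wheel rotation toward either end of a clamped range.
; Each tick also eases yaw, pitch and roll differences from FlyingHandler at a constant rate, then writes them, some scaled, to flap rotators for the AnimBP.
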(event `self.ReceiveBeginPlay`
  (set `self.AnimBlueprint` (cast `/Game/Animations/G_PlaneAnimBP` (`SkeletalMeshComponent.GetAnimInstance` (`self.AircraftMesh`)) :!pure true)))

(event `self.ReceiveTick`
  (params (DeltaSeconds :type "Float (single-precision)"))
  (`self.HandleGearBoneRotation` DeltaSeconds)
  (`self.HandleFlapRotations` DeltaSeconds))

(event `self.OnOffGears`
  (bind _isa (`/Engine/EditorBlueprintResources/StandardMacros.FlipFlop`)
    (:`A`
      _)
    (:`B`
      _))
  (set `self.IsGearsOn` _isa))

(fn `HandleFlapRotations`
  (params (DeltaTime :type "Float (double-precision)"))
  (bind _flyinghandler (`self.FlyingHandler`))
  (bind _animblueprint (`self.AnimBlueprint`))
  (`|ExecutionSequence`
    (:`then_0`
      (bind _output_get (set `self.CurrentYaw` (`KismetMathLibrary.FInterpTo_Constant` (`self.CurrentYaw`) (`FlyingHandler.GetYawDifference` _flyinghandler) DeltaTime 50.0)))
      (set `/Game/Animations/G_PlaneAnimBP.YawRotator` (`KismetMathLibrary.MakeRotator` 0.0 0.0 _output_get) _animblueprint))
    (:`then_1`
      (bind _output_get_2 (set `self.CurrentPitch` (`KismetMathLibrary.FInterpTo_Constant` (`self.CurrentPitch`) (`FlyingHandler.GetPitchDifference` _flyinghandler) DeltaTime 50.0)))
      (set `/Game/Animations/G_PlaneAnimBP.PitchRotator` (`KismetMathLibrary.MakeRotator` 0.0 (* _output_get_2 1.25)) _animblueprint))
    (:`then_2`
      (bind _output_get_3 (set `self.CurrentRoll` (`KismetMathLibrary.FInterpTo_Constant` (`self.CurrentRoll`) (`FlyingHandler.GetRollDifference` _flyinghandler) DeltaTime 50.0)))
      (set `/Game/Animations/G_PlaneAnimBP.ElevatorFlapRotator` (`KismetMathLibrary.MakeRotator` 0.0 (* _output_get_3 0.75)) _animblueprint))))

(fn `HandleGearBoneRotation`
  (params (DeltaSeconds :type "Float (double-precision)"))
  (bind _animblueprint (`self.AnimBlueprint`))
  (bind _wheelsrotation_roll (`KismetMathLibrary.BreakRotator` (`/Game/Animations/G_PlaneAnimBP.WheelsRotation` _animblueprint)))
  (if (`self.IsGearsOn`)
    (set `/Game/Animations/G_PlaneAnimBP.WheelsRotation` (`KismetMathLibrary.MakeRotator` (`KismetMathLibrary.FClamp` (+ (* DeltaSeconds 10.0) _wheelsrotation_roll) 0.0 80.0)) _animblueprint)
    (else
      (set `/Game/Animations/G_PlaneAnimBP.WheelsRotation` (`KismetMathLibrary.MakeRotator` (`KismetMathLibrary.FClamp` (- _wheelsrotation_roll (* DeltaSeconds 10.0)) 0.0 80.0)) _animblueprint))))

(fn `UserConstructionScript`)